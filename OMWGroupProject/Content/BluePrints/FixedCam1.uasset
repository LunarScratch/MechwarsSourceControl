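; Fixed-position camera actor that rotates in place to keep facing player 0's pawn.
; BeginPlay points it straight at the pawn using a rotation built from the direction vector.
; Tick computes a look-at rotation and feeds it through RInterpTo with no interp speed specified.
; Both events write world-space rotations through SetActorRelativeRotation.
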(event `self.ReceiveBeginPlay`
  (`self.K2_SetActorRelativeRotation` (`KismetMathLibrary.Conv_VectorToRotator` (- (`self.K2_GetActorLocation` (`GameplayStatics.GetPlayerPawn` 0)) (`self.K2_GetActorLocation`)))))

(event `self.ReceiveTick`
  (params (DeltaSeconds :type "Float (single-precision)"))
  (`self.K2_SetActorRelativeRotation` (`KismetMathLibrary.RInterpTo` (`self.K2_GetActorRotation`) (`KismetMathLibrary.FindLookAtRotation` (`self.K2_GetActorLocation`) (`self.K2_GetActorLocation` (`GameplayStatics.GetPlayerPawn` 0))) DeltaSeconds)))

(fn `UserConstructionScript`)