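; BP_Book2 is a clickable puzzle book about Famine, collectable only after the player's Book1 flag is set.
; Hovering swaps the cube to a highlighted material, and clicking shows a typewriter text description that removes itself after finishing.
; The box overlap toggles input for BP_MyChar_2, so pressing Interaction checks Book1, then either sets Book2 with a click sound or plays a failure sound.
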(event `self.ReceiveActorOnClicked`
  (params (ButtonPressed :type "Key Structure"))
  ;[1 1 1] Clicked Event
  (bind _returnvalue (`|CreateWidget` "/Game/BluePrints/UI/WB_TypewriterTextBox.WB_TypewriterTextBox_C" (cast `PlayerController` (`GameplayStatics.GetPlayerController` 0) :!pure true) 20.0))
  (`UserWidget.AddToViewport` _returnvalue 0)
  (`/Game/BluePrints/UI/WB_TypewriterTextBox.Write` _returnvalue "A book about Famine (press E to interact)")
  (add `/Game/BluePrints/UI/WB_TypewriterTextBox.FinishedWriting` _returnvalue (delegate `FinishedWriting_Event_0`)))

(event `FinishedWriting_Event_0`
  ;[1 1 1] Clicked Event
  (`KismetSystemLibrary.Delay` 2.0)
  (`Widget.RemoveFromParent` (stale `self.ReceiveActorOnClicked` _returnvalue)))

(event `self.Box.OnComponentBeginOverlap`
  (params (OverlappedComponent :type "PrimitiveComponent Object Reference") (OtherActor :type "Actor Object Reference") (OtherComp :type "PrimitiveComponent Object Reference") (OtherBodyIndex :type Integer) (bFromSweep :type Boolean) (SweepResult :type "HitResult Structure (by ref)"))
  (cast `/Game/Character/BP_MyChar_2` OtherActor)
  (`self.EnableInput` (`GameplayStatics.GetPlayerController` 0)))

(event `self.Box.OnComponentEndOverlap`
  (params (OverlappedComponent :type "PrimitiveComponent Object Reference") (OtherActor :type "Actor Object Reference") (OtherComp :type "PrimitiveComponent Object Reference") (OtherBodyIndex :type Integer))
  (cast `/Game/Character/BP_MyChar_2` OtherActor)
  (`self.DisableInput` (`GameplayStatics.GetPlayerController` 0)))

(event `InputAction|Interaction`
  (params (Key :type "Key Structure"))
  (bind _returnvalue (`self.K2_GetActorLocation` (`GameplayStatics.GetPlayerCharacter` 0)))
  (:`Pressed`
    (bind _asbp_my_char_2 (cast `/Game/Character/BP_MyChar_2` (stale `self.Box.OnComponentBeginOverlap` OtherActor)))
    (if (`/Game/Character/BP_MyChar_2.bBook1` _asbp_my_char_2)
      (set `/Game/Character/BP_MyChar_2.bBook2` true _asbp_my_char_2)
      (`GameplayStatics.PlaySoundAtLocation` "/Engine/VREditor/Sounds/UI/Click_on_Button_Cue.Click_on_Button_Cue" _returnvalue (struct) 1.0 1.0 0.0 null null null null)
      (else
        (`GameplayStatics.PlaySoundAtLocation` "/Engine/EditorSounds/Notifications/CompileFailed.CompileFailed" _returnvalue (struct) 1.0 1.0 0.0 null null null null)))))

(event `self.ReceiveActorBeginCursorOver`
  ;[1 1 1] Hover Event
  (`PrimitiveComponent.SetMaterial` (`self.Cube`) 0 "/Game/Materials/JN_PuzzleBookGreenHighlighted.JN_PuzzleBookGreenHighlighted"))

(event `self.ReceiveActorEndCursorOver`
  ;[1 1 1] If you stop hovering over obejct, it returns to normal
  (`PrimitiveComponent.SetMaterial` (`self.Cube`) 0 "/Game/Materials/JN_PuzzleBookGreen.JN_PuzzleBookGreen"))

(fn `UserConstructionScript`)