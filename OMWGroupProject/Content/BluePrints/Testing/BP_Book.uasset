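; BP_Book is a testing book pickup or switch that toggles the Book1 flag on the BP_MyChar_2 character.
; Its Box overlap enables player input on the book while that character is inside and disables it on exit.
; Pressing Interaction flips the flag and plays a different sound at the player's location for each state.
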(event `self.Box.OnComponentBeginOverlap`
  (params (OverlappedComponent :type "PrimitiveComponent Object Reference") (OtherActor :type "Actor Object Reference") (OtherComp :type "PrimitiveComponent Object Reference") (OtherBodyIndex :type Integer) (bFromSweep :type Boolean) (SweepResult :type "HitResult Structure (by ref)"))
  (cast `/Game/Character/BP_MyChar_2` OtherActor)
  (`self.EnableInput` (`GameplayStatics.GetPlayerController` 0)))

(event `self.Box.OnComponentEndOverlap`
  (params (OverlappedComponent :type "PrimitiveComponent Object Reference") (OtherActor :type "Actor Object Reference") (OtherComp :type "PrimitiveComponent Object Reference") (OtherBodyIndex :type Integer))
  (cast `/Game/Character/BP_MyChar_2` OtherActor)
  (`self.DisableInput` (`GameplayStatics.GetPlayerController` 0)))

(event `InputAction|Interaction`
  (params (Key :type "Key Structure"))
  (bind _returnvalue (`self.K2_GetActorLocation` (`GameplayStatics.GetPlayerCharacter` 0)))
  (:`Pressed`
    (bind _asbp_my_char_2 (cast `/Game/Character/BP_MyChar_2` (stale `self.Box.OnComponentBeginOverlap` OtherActor)))
    (if (`/Game/Character/BP_MyChar_2.bBook1` _asbp_my_char_2)
      (set `/Game/Character/BP_MyChar_2.bBook1` false _asbp_my_char_2)
      (`GameplayStatics.PlaySoundAtLocation` "/Engine/EditorSounds/Notifications/CompileFailed.CompileFailed" _returnvalue (struct) 1.0 1.0 0.0 null null null null)
      (else
        (set `/Game/Character/BP_MyChar_2.bBook1` true _asbp_my_char_2)
        (`GameplayStatics.PlaySoundAtLocation` "/Engine/VREditor/Sounds/UI/Click_on_Button_Cue.Click_on_Button_Cue" _returnvalue (struct) 1.0 1.0 0.0 null null null null)))))

(fn `UserConstructionScript`)