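; MechSuit is a clickable test actor representing a mech suit that shows a line of dialogue when clicked.
; Cursor hover swaps the mesh's first material to a highlighted instance and restores it when the cursor leaves.
; A click creates a typewriter text box widget that writes a fixed message, then removes it after a short delay once its finished-writing event fires.
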(event `self.ReceiveActorOnClicked`
  (params (ButtonPressed :type "Key Structure"))
  ;[1 1 1] Clicked Event
  (bind _returnvalue (`|CreateWidget` "/Game/BluePrints/UI/WB_TypewriterTextBox.WB_TypewriterTextBox_C" (cast `PlayerController` (`GameplayStatics.GetPlayerController` 0) :!pure true) 20.0))
  (`UserWidget.AddToViewport` _returnvalue 0)
  (`/Game/BluePrints/UI/WB_TypewriterTextBox.Write` _returnvalue "Don't worry bro. I'll bring you back...")
  (add `/Game/BluePrints/UI/WB_TypewriterTextBox.FinishedWriting` _returnvalue (delegate `FinishedWriting_Event_0`)))

(event `FinishedWriting_Event_0`
  ;[1 1 1] Clicked Event
  (`KismetSystemLibrary.Delay` 2.0)
  (`Widget.RemoveFromParent` (stale `self.ReceiveActorOnClicked` _returnvalue)))

(event `self.ReceiveActorBeginCursorOver`
  ;[1 1 1] Hover Event
  (`PrimitiveComponent.SetMaterial` (`self.MechSuit`) 0 "/Game/Materials/MI_MechSuitHighlieghted.MI_MechSuitHighlieghted"))

(event `self.ReceiveActorEndCursorOver`
  ;[1 1 1] If you stop hovering over obejct, it returns to normal
  (`PrimitiveComponent.SetMaterial` (`self.MechSuit`) 0 "/Game/Materials/MI_MechSuit.MI_MechSuit"))

(fn `UserConstructionScript`)