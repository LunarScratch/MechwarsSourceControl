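; BP_MyChar is a test player character Blueprint that handles basic look and movement input.
; Four axis events drive it: the look axes feed controller yaw and pitch, and the move axes feed AddMovementInput.
; Movement directions come from the Mesh component's forward and right vectors rather than the control rotation.
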(event `InputAxis|Look Right/Left`
  (params (AxisValue :type "Float (single-precision)"))
  (`self.AddControllerYawInput` AxisValue))

(event `InputAxis|Look Up/down`
  (params (AxisValue :type "Float (single-precision)"))
  (`self.AddControllerPitchInput` AxisValue))

(event `InputAxis|Move Forward/Backwards`
  (params (AxisValue :type "Float (single-precision)"))
  (`self.AddMovementInput` (`SceneComponent.GetForwardVector` (`self.Mesh`)) AxisValue))

(event `InputAxis|Move Left/Right`
  (params (AxisValue :type "Float (single-precision)"))
  (`self.AddMovementInput` (`SceneComponent.GetRightVector` (`self.Mesh`)) AxisValue))

(fn `UserConstructionScript`)