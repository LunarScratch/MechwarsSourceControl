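; BP_Book3 is a test puzzle book, the third step in an ordered three-book interaction sequence.
; A box overlap with BP_MyChar_2 toggles input; Interaction sets the character's Book3 flag if Book1 and Book2 are set, otherwise clears those two, with a sound for each outcome.
; Cursor hover swaps to a highlighted material.
; Clicking shows a placeholder typewriter text box that removes itself shortly after it finishes writing.
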(event `self.ReceiveActorOnClicked`
  (params (ButtonPressed :type "Key Structure"))
  ;[1 1 1] Clicked Event
  (bind _returnvalue (`|CreateWidget` "/Game/BluePrints/UI/WB_TypewriterTextBox.WB_TypewriterTextBox_C" (cast `PlayerController` (`GameplayStatics.GetPlayerController` 0) :!pure true) 20.0))
  (`UserWidget.AddToViewport` _returnvalue 0)
  (`/Game/BluePrints/UI/WB_TypewriterTextBox.Write` _returnvalue "A working text box! Our game is making progress!")
  (add `/Game/BluePrints/UI/WB_TypewriterTextBox.FinishedWriting` _returnvalue (delegate `FinishedWriting_Event_0`)))

(event `FinishedWriting_Event_0`
  ;[1 1 1] Clicked Event
  (`KismetSystemLibrary.Delay` 2.0)
  (`Widget.RemoveFromParent` (stale `self.ReceiveActorOnClicked` _returnvalue)))

(event `self.Box.OnComponentBeginOverlap`
  (params (OverlappedComponent :type "PrimitiveComponent Object Reference") (OtherActor :type "Actor Object Reference") (OtherComp :type "PrimitiveComponent Object Reference") (OtherBodyIndex :type Integer) (bFromSweep :type Boolean) (SweepResult :type "HitResult Structure (by ref)"))
  (cast `/Game/Character/BP_MyChar_2` OtherActor)
  (`self.EnableInput` (`GameplayStatics.GetPlayerController` 0)))

(event `self.Box.OnComponentEndOverlap`
  (params (OverlappedComponent :type "PrimitiveComponent Object Reference") (OtherActor :type "Actor Object Reference") (OtherComp :type "PrimitiveComponent Object Reference") (OtherBodyIndex :type Integer))
  (cast `/Game/Character/BP_MyChar_2` OtherActor)
  (`self.DisableInput` (`GameplayStatics.GetPlayerController` 0)))

(event `InputAction|Interaction`
  (params (Key :type "Key Structure"))
  (:`Pressed`
    (bind _asbp_my_char_2 (cast `/Game/Character/BP_MyChar_2` (stale `self.Box.OnComponentBeginOverlap` OtherActor)))
    (if (`/Game/Character/BP_MyChar_2.bBook1` _asbp_my_char_2)
      (if (`/Game/Character/BP_MyChar_2.bBook2` _asbp_my_char_2)
        (set `/Game/Character/BP_MyChar_2.bBook3` true _asbp_my_char_2)
        (`GameplayStatics.PlaySoundAtLocation` "/Engine/VREditor/Sounds/UI/Click_on_Button.Click_on_Button" (`self.K2_GetActorLocation` _asbp_my_char_2) (struct) 1.0 1.0 0.0 null null null null)
        (else
          (set `/Game/Character/BP_MyChar_2.bBook2` false _asbp_my_char_2 :!label _label)
          (set `/Game/Character/BP_MyChar_2.bBook1` false _asbp_my_char_2)
          (`GameplayStatics.PlaySoundAtLocation` "/Engine/EditorSounds/Notifications/CompileFailed.CompileFailed" (`self.K2_GetActorLocation` _asbp_my_char_2) (struct) 1.0 1.0 0.0 null null null null)))
      (else
        (goto _label)))))

(event `self.ReceiveActorBeginCursorOver`
  ;[1 1 1] Hover Event
  (`PrimitiveComponent.SetMaterial` (`self.Cube`) 0 "/Game/Materials/JN_PuzzleBookPurpleHighlighted.JN_PuzzleBookPurpleHighlighted"))

(event `self.ReceiveActorEndCursorOver`
  ;[1 1 1] If you stop hovering over obejct, it returns to normal
  (`PrimitiveComponent.SetMaterial` (`self.Cube`) 0 "/Game/Materials/JN_PuzzleBookPurple.JN_PuzzleBookPurple"))

(fn `UserConstructionScript`)