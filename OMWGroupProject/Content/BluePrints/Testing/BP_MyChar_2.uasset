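; Test player character that combines control-yaw-relative axis movement with click-to-move toward pawns under the cursor.
; Holding left mouse opens a Tick gate that traces for a Pawn each frame and calls SimpleMoveToActor, or prints a debug "Hello" when none is hit.
; BeginPlay enables click and mouse-over events.
; An unused click-to-point path would set walk speed by distance and move to the cursor location.
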(event `InputAxis|Move Forward/Backwards`
  (params (AxisValue :type "Float (single-precision)"))
  ;[1 1 1] Movement
  (`self.AddMovementInput` (`KismetMathLibrary.GetForwardVector` (`KismetMathLibrary.MakeRotator` 0.0 0.0 (.yaw (`self.GetControlRotation`)))) AxisValue))

(event `InputAxis|Move Left/Right`
  (params (AxisValue :type "Float (single-precision)"))
  ;[1 1 1] Movement
  (`self.AddMovementInput` (`KismetMathLibrary.GetRightVector` (`KismetMathLibrary.MakeRotator` 0.0 0.0 (.yaw (`self.GetControlRotation`)))) AxisValue))

(event `self.ReceiveBeginPlay`
  (bind _returnvalue (`GameplayStatics.GetPlayerController` 0))
  ;[1 1 1] Interacting with objects
  (set `PlayerController.bEnableClickEvents` true _returnvalue)
  (set `PlayerController.bEnableMouseOverEvents` true _returnvalue))

(event `self.ReceiveTick`
  (params (DeltaSeconds :type "Float (single-precision)"))
  (`/Engine/EditorBlueprintResources/StandardMacros.Gate` true :!label _label
    (:`Exit`
      (bind _clicked_actor (`self.Get Clicked Actor`))
      (`/Engine/EditorBlueprintResources/StandardMacros.IsValid` _clicked_actor
        (:`Is Valid`
          (`self.Move to actor` _clicked_actor))
        (:`Is Not Valid`
          (`KismetSystemLibrary.PrintString` "Hello"))))))

(event `Key|LeftMouseButton`
  (params (Key :type "Key Structure"))
  (:`Pressed`
    (goto _label :!via `Open`))
  (:`Released`
    (goto _label :!via `Close`)))

(fn `Get Clicked Actor`
  (returns (`Clicked Actor` :type "Actor Object Reference"))
  (return (`.HitActor` (`GameplayStatics.BreakHitResult` (`PlayerController.GetHitResultUnderCursorForObjects` (`GameplayStatics.GetPlayerController` 0) (`|MakeArray` "ObjectTypeQuery3" :!type "EObjectTypeQuery Enum") true)))))

(fn `Get Destiniation To Move`
  (returns (`Destination ` :type "Vector Structure"))
  (return (`.Location` (`GameplayStatics.BreakHitResult` (`PlayerController.GetHitResultUnderCursorByChannel` (`GameplayStatics.GetPlayerController` 0) "TraceTypeQuery1" true)))))

(fn `Move to actor`
  (params (`Move to actor` :type "Actor Object Reference"))
  (`AIBlueprintHelperLibrary.SimpleMoveToActor` (`GameplayStatics.GetPlayerController` 0) `Move to actor`))

(fn `Move To Clicked Point`
  (locals (`Move Destination ` :type "Vector Structure"))
  (bind _charactermovement (`self.CharacterMovement`))
  (bind _destination_ (`self.Get Destiniation To Move`))
  (set `local.Move Destination ` _destination_)
  (if (> (`KismetMathLibrary.VSize` (- (`local.Move Destination `) (`self.K2_GetActorLocation`))) 150.0)
    (set `CharacterMovementComponent.MaxWalkSpeed` 600.0 _charactermovement)
    (else
      (set `CharacterMovementComponent.MaxWalkSpeed` 150.0 _charactermovement)))
  (`AIBlueprintHelperLibrary.SimpleMoveToLocation` (`GameplayStatics.GetPlayerController` 0) (`local.Move Destination `)))

(fn `UserConstructionScript`)