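; BP_Book4 is an interactable book that acts as the fourth step in an ordered book sequence for BP_MyChar_2.
; Its Box overlap enables and disables player input, so the Interaction action only responds while the character is near.
; On press, if the character's Book1 to Book3 flags are all set, it sets Book4 and plays a click.
; Otherwise it clears those three flags and plays a failure sound.
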(event `self.Box.OnComponentBeginOverlap`
  (params (OverlappedComponent :type "PrimitiveComponent Object Reference") (OtherActor :type "Actor Object Reference") (OtherComp :type "PrimitiveComponent Object Reference") (OtherBodyIndex :type Integer) (bFromSweep :type Boolean) (SweepResult :type "HitResult Structure (by ref)"))
  (cast `/Game/Character/BP_MyChar_2` OtherActor)
  (`self.EnableInput` (`GameplayStatics.GetPlayerController` 0)))

(event `self.Box.OnComponentEndOverlap`
  (params (OverlappedComponent :type "PrimitiveComponent Object Reference") (OtherActor :type "Actor Object Reference") (OtherComp :type "PrimitiveComponent Object Reference") (OtherBodyIndex :type Integer))
  (cast `/Game/Character/BP_MyChar_2` OtherActor)
  (`self.DisableInput` (`GameplayStatics.GetPlayerController` 0)))

(event `InputAction|Interaction`
  (params (Key :type "Key Structure"))
  (:`Pressed`
    (bind _asbp_my_char_2 (cast `/Game/Character/BP_MyChar_2` (stale `self.Box.OnComponentBeginOverlap` OtherActor)))
    (if (`/Game/Character/BP_MyChar_2.bBook1` _asbp_my_char_2)
      (if (`/Game/Character/BP_MyChar_2.bBook2` _asbp_my_char_2)
        (if (`/Game/Character/BP_MyChar_2.bBook3` _asbp_my_char_2)
          (set `/Game/Character/BP_MyChar_2.bBook4` true _asbp_my_char_2)
          (`GameplayStatics.PlaySoundAtLocation` "/Engine/VREditor/Sounds/UI/Click_on_Button.Click_on_Button" (`self.K2_GetActorLocation` _asbp_my_char_2) (struct) 1.0 1.0 0.0 null null null null)
          (else
            (set `/Game/Character/BP_MyChar_2.bBook2` false _asbp_my_char_2 :!label _label)
            (set `/Game/Character/BP_MyChar_2.bBook1` false _asbp_my_char_2)
            (set `/Game/Character/BP_MyChar_2.bBook3` false _asbp_my_char_2)
            (`GameplayStatics.PlaySoundAtLocation` "/Engine/EditorSounds/Notifications/CompileFailed.CompileFailed" (`self.K2_GetActorLocation` _asbp_my_char_2) (struct) 1.0 1.0 0.0 null null null null)))
        (else
          (goto _label)))
      (else
        (goto _label)))))

(fn `UserConstructionScript`)