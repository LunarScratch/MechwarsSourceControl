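; Clickable door actor that teleports the player character, by its name from the garage to the living room.
; On click, it sets the character's root to the TeleportLocation component's world transform and plays a door sound at the world origin.
; Cursor hover swaps the door mesh between highlighted and normal materials.
; The construction script positions TeleportLocation from the TeleporterLocation transform variable, relative to its parent.
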(event `self.ReceiveActorOnClicked`
  (params (ButtonPressed :type "Key Structure"))
  ;[1 1 1] Clicked Event
  (`SceneComponent.K2_SetWorldTransform` (`Actor.RootComponent` (`GameplayStatics.GetPlayerCharacter` 0)) (`SceneComponent.K2_GetComponentToWorld` (`self.Teleport Location`)) false false)
  (`GameplayStatics.PlaySoundAtLocation` "/Game/Audio/SoundEffects/DoorSoundEffect.DoorSoundEffect" (0.0 0.0 0.0) (struct) 1.0 1.0 0.0 null null null null))

(event `self.ReceiveActorBeginCursorOver`
  ;[1 1 1] Hover Event
  (`PrimitiveComponent.SetMaterial` (`self.JN_Door`) 0 "/Game/Materials/JN_DoorHighlighted.JN_DoorHighlighted"))

(event `self.ReceiveActorEndCursorOver`
  ;[1 1 1] If you stop hovering over obejct, it returns to normal
  (`PrimitiveComponent.SetMaterial` (`self.JN_Door`) 0 "/Game/Materials/JN_Door.JN_Door"))

(fn `UserConstructionScript`
  (`SceneComponent.K2_SetRelativeTransform` (`self.Teleport Location`) (`self.Teleporter Location`) false false))