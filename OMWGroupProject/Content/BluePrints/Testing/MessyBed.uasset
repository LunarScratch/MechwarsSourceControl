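; MessyBed is a clickable bed prop that shows a character thought about making the bed later.
; Hovering swaps the Bed mesh to a highlighted material instance and restores the normal one when the cursor leaves.
; Clicking creates a WB_TypewriterTextBox widget that types the line, then removes it after a short delay once its FinishedWriting event fires.
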(event `self.ReceiveActorOnClicked`
  (params (ButtonPressed :type "Key Structure"))
  ;[1 1 1] Clicked Event
  (bind _returnvalue (`|CreateWidget` "/Game/BluePrints/UI/WB_TypewriterTextBox.WB_TypewriterTextBox_C" (cast `PlayerController` (`GameplayStatics.GetPlayerController` 0) :!pure true) 20.0))
  (`UserWidget.AddToViewport` _returnvalue 0)
  (`/Game/BluePrints/UI/WB_TypewriterTextBox.Write` _returnvalue "I should make my bed later...")
  (add `/Game/BluePrints/UI/WB_TypewriterTextBox.FinishedWriting` _returnvalue (delegate `FinishedWriting_Event_0`)))

(event `FinishedWriting_Event_0`
  ;[1 1 1] Clicked Event
  (`KismetSystemLibrary.Delay` 2.0)
  (`Widget.RemoveFromParent` (stale `self.ReceiveActorOnClicked` _returnvalue)))

(event `self.ReceiveActorBeginCursorOver`
  ;[1 1 1] Hover Event
  (`PrimitiveComponent.SetMaterial` (`self.Bed`) 0 "/Game/Materials/MI_Bed_Highlighted.MI_Bed_Highlighted"))

(event `self.ReceiveActorEndCursorOver`
  ;[1 1 1] If you stop hovering over obejct, it returns to normal
  (`PrimitiveComponent.SetMaterial` (`self.Bed`) 0 "/Game/Materials/MI_Bed.MI_Bed"))

(fn `UserConstructionScript`)