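; BP_Desktop is a test interactable desktop computer actor with monitor highlighting, typewriter text and video playback.
; Cursor hover swaps the monitor material, and clicking shows a WB_TypewriterTextBox message that removes itself shortly after writing finishes.
; Overlapping the box starts the media source with sound, then hides Plane1 after a short delay.
; Interact1 switches Plane to a video material and opens the Data_Encrypting source.
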(event `self.ReceiveActorOnClicked`
  (params (ButtonPressed :type "Key Structure"))
  ;[1 1 1] Clicked Event
  (bind _returnvalue (`|CreateWidget` "/Game/BluePrints/UI/WB_TypewriterTextBox.WB_TypewriterTextBox_C" (`GameplayStatics.GetPlayerController` 0) 20.0))
  (`UserWidget.AddToViewport` _returnvalue 0)
  (`/Game/BluePrints/UI/WB_TypewriterTextBox.Write` _returnvalue "Death, Famine, War, and Conquest")
  (add `/Game/BluePrints/UI/WB_TypewriterTextBox.FinishedWriting` _returnvalue (delegate `FinishedWriting_Event_0`)))

(event `FinishedWriting_Event_0`
  ;[1 1 1] Clicked Event
  (`KismetSystemLibrary.Delay` 2.0)
  (`Widget.RemoveFromParent` (stale `self.ReceiveActorOnClicked` _returnvalue)))

(event `self.ReceiveActorBeginCursorOver`
  ;[1 1 1] Hover Event
  (`PrimitiveComponent.SetMaterial` (`self.Monitor`) 0 "/Game/Materials/MI_MonitorHighlighted.MI_MonitorHighlighted"))

(event `self.ReceiveActorEndCursorOver`
  ;[1 1 1] If you stop hovering over obejct, it returns to normal
  (`PrimitiveComponent.SetMaterial` (`self.Monitor`) 0 "/Game/Materials/MI_Monitor.MI_Monitor"))

(event `self.Box.OnComponentBeginOverlap`
  (params (OverlappedComponent :type "PrimitiveComponent Object Reference") (OtherActor :type "Actor Object Reference") (OtherComp :type "PrimitiveComponent Object Reference") (OtherBodyIndex :type Integer) (bFromSweep :type Boolean) (SweepResult :type "HitResult Structure (by ref)"))
  ;[1 1 1] Video component
  (`MediaPlayer.OpenSource` (`self.MediaPlayer`) (`self.Media Source`))
  (`MediaSoundComponent.SetMediaPlayer` (`self.MediaSound`) (`self.MediaPlayer`))
  (`KismetSystemLibrary.Delay` 0.5)
  (`SceneComponent.SetVisibility` (`self.Plane1`) false false))

(event `/Game/BluePrints/Interact_Interface1.Interact 1`
  (`PrimitiveComponent.SetMaterial` (`self.Plane`) 0 "/Game/Movies/Desktop_Player_Video_Mat.Desktop_Player_Video_Mat")
  (`MediaPlayer.OpenSource` (`self.MediaPlayer`) "/Game/Movies/Data_Encrypting.Data_Encrypting"))

(event `self.Plane.OnComponentBeginOverlap`
  (params (OverlappedComponent :type "PrimitiveComponent Object Reference") (OtherActor :type "Actor Object Reference") (OtherComp :type "PrimitiveComponent Object Reference") (OtherBodyIndex :type Integer) (bFromSweep :type Boolean) (SweepResult :type "HitResult Structure (by ref)")))

(event `OnActorEndOverlap_Event` :!signature `self.OnActorEndOverlap`
  (params (OverlappedActor :type "Actor Object Reference") (OtherActor :type "Actor Object Reference")))

(fn `UserConstructionScript`)