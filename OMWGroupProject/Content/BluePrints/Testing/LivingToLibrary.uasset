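; LivingToLibrary is a clickable door actor, kept in a testing folder, that teleports the player between areas, apparently from the living room to the library.
; Clicking it moves player 0's character root to the world transform of the TeleportLocation reference.
; Hovering the cursor swaps the JNDoor material to a green highlight, and leaving restores the normal door material.
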(event `self.ReceiveActorOnClicked`
  (params (ButtonPressed :type "Key Structure"))
  ;[1 1 1] Clicked Event
  (`SceneComponent.K2_SetWorldTransform` (`Actor.RootComponent` (`GameplayStatics.GetPlayerCharacter` 0)) (`SceneComponent.K2_GetComponentToWorld` (`self.Teleport Location`)) false false))

(event `self.ReceiveActorBeginCursorOver`
  ;[1 1 1] Hover Event
  (`PrimitiveComponent.SetMaterial` (`self.JN_Door`) 0 "/Engine/EngineDebugMaterials/VertexColorViewMode_GreenOnly.VertexColorViewMode_GreenOnly"))

(event `self.ReceiveActorEndCursorOver`
  ;[1 1 1] If you stop hovering over obejct, it returns to normal
  (`PrimitiveComponent.SetMaterial` (`self.JN_Door`) 0 "/Game/Materials/JN_Door.JN_Door"))

(fn `UserConstructionScript`)