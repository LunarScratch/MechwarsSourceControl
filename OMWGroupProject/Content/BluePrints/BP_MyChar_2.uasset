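; BP_MyChar_2 is a player character Blueprint that handles basic movement and enables mouse interaction with objects.
; Forward/backward and left/right axis inputs add movement along directions derived from the control rotation's yaw only, keeping movement independent of pitch and roll.
; On BeginPlay it enables click and mouse-over events on player controller 0.
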(event `InputAxis|Move Forward/Backwards`
  (params (AxisValue :type "Float (single-precision)"))
  ;[1 1 1] Movement
  (`self.AddMovementInput` (`KismetMathLibrary.GetForwardVector` (`KismetMathLibrary.MakeRotator` 0.0 0.0 (.yaw (`self.GetControlRotation`)))) AxisValue))

(event `InputAxis|Move Left/Right`
  (params (AxisValue :type "Float (single-precision)"))
  ;[1 1 1] Movement
  (`self.AddMovementInput` (`KismetMathLibrary.GetRightVector` (`KismetMathLibrary.MakeRotator` 0.0 0.0 (.yaw (`self.GetControlRotation`)))) AxisValue))

(event `self.ReceiveBeginPlay`
  (bind _returnvalue (`GameplayStatics.GetPlayerController` 0))
  ;[1 1 1] Interacting with objects
  (set `PlayerController.bEnableClickEvents` true _returnvalue)
  (set `PlayerController.bEnableMouseOverEvents` true _returnvalue))

(fn `UserConstructionScript`)