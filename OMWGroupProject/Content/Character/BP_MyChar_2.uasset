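; BP_MyChar_2 is a player character with yaw-relative axis movement and a four-book puzzle check.
; Forward and strafe inputs derive their directions from the control rotation's yaw.
; BeginPlay enables click and mouse-over events on the player controller for object interaction.
; Tick sets Puzzle1 once all four Book flags are true, calling PlaySoundAtLocation at the character every frame while they remain true.
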(event `InputAxis|Move Forward/Backwards`
  (params (AxisValue :type "Float (single-precision)"))
  ;[1 1 1] Movement
  (`self.AddMovementInput` (`KismetMathLibrary.GetForwardVector` (`KismetMathLibrary.MakeRotator` 0.0 0.0 (.yaw (`self.GetControlRotation`)))) AxisValue))

(event `InputAxis|Move Left/Right`
  (params (AxisValue :type "Float (single-precision)"))
  ;[1 1 1] Movement
  (`self.AddMovementInput` (`KismetMathLibrary.GetRightVector` (`KismetMathLibrary.MakeRotator` 0.0 0.0 (.yaw (`self.GetControlRotation`)))) AxisValue))

(event `self.ReceiveBeginPlay`
  (bind _returnvalue (`GameplayStatics.GetPlayerController` 0))
  ;[1 1 1] Interacting with objects
  (set `PlayerController.bEnableClickEvents` true _returnvalue)
  (set `PlayerController.bEnableMouseOverEvents` true _returnvalue))

(event `self.ReceiveTick`
  (params (DeltaSeconds :type "Float (single-precision)"))
  (if (`self.bBook1`)
    (if (`self.bBook2`)
      (if (`self.bBook3`)
        (if (`self.bBook4`)
          (set `self.bPuzzle1` true)
          (`GameplayStatics.PlaySoundAtLocation` null (`self.K2_GetActorLocation`) (struct) 1.0 1.0 0.0 null null null null))))))

(fn `UserConstructionScript`)